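; BP_EnemyLight is a moving puzzle enemy that sends the player's mesh back near the world origin on contact.
; On BeginPlay, a timeline scaled by TimeToComplete moves and rotates the actor along its spline's length.
; Spline samples are in local space but are applied as the actor's transform.
; When a BP_Pawn overlaps the Box, its PlayerMesh is moved to a hardcoded world position.
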(event OnComponentBeginOverlap(Box)
  (params (OverlappedComponent :type Primitive%20Component%20Object%20Reference) (OtherActor :type Actor%20Object%20Reference) (OtherComp :type Primitive%20Component%20Object%20Reference) (OtherBodyIndex :type Integer) (bFromSweep :type Boolean) (SweepResult :type Hit%20Result%20Structure%20%28by%20ref%29))
  (bind _asbp_pawn (Utilities|Casting|CastToBP_Pawn OtherActor))
  (Utilities|IsValid _asbp_pawn
    (:Is%20Valid
      (Transformation|SetWorldLocation (Variables|/Script/Project_1.Project_1Pawn|GetPlayerMesh _asbp_pawn) "0.000000,0.000000,1.000000" false false))))

(event Custom|Move%20Object
  (bind _spline (Variables|Default|GetSpline))
  (Components|Timeline|SetPlayRate (Variables|Default|GetMove%20Object%20T) (/ 1.0 (Variables|Default|GetTime%20To%20Complete)))
  (bind _move_track (Timeline|Move%20Object%20T PlayFromStart)
    (:Update
      (Transformation|SetActorTransform (Math|Transform|MakeTransform (Spline|GetLocationatDistanceAlongSpline _spline (Math|Float|Lerp 0.0 (Spline|GetSplineLength (Variables|Default|GetSpline)) _move_track) "Local") (Spline|GetRotationatDistanceAlongSpline _spline (Math|Float|Lerp 0.0 (Spline|GetSplineLength (Variables|Default|GetSpline)) _move_track) "Local") "1.000000,1.000000,1.000000")))))

(event EventBeginPlay
  (CallFunction|MoveObject))

(fn ConstructionScript)