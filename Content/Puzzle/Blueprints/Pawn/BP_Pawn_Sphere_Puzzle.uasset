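; Puzzle sphere pawn that moves on axis input and visually rolls its ball mesh.
; MoveX and MoveY feed AddMovementInput with speed-scaled forward and right vectors; zeroed control yaw keeps these directions fixed to world axes.
; The movement component updates PlayerMesh, which Tick rotates around an axis perpendicular to velocity, by an angle proportional to speed and frame time.
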(event EventBeginPlay
  (|CallParentFunction)
  (Components|Movement|SetUpdatedComponent (Variables|Default|GetPawnMovementComponent) (Variables|Default|GetPlayerMesh)))

(event EventTick
  (params (DeltaSeconds :type Float%20%28single-precision%29))
  (CallFunction|RotateBallMesh DeltaSeconds))

(event Input|AxisEvents|InputAxisMoveX
  (params (AxisValue :type Float%20%28single-precision%29))
  (CallFunction|MoveForwardorBack AxisValue))

(event Input|AxisEvents|InputAxisMoveY
  (params (AxisValue :type Float%20%28single-precision%29))
  (CallFunction|MoveRightorLeft AxisValue))

(fn ConstructionScript
  (|CallParentFunction))

(fn MoveForwardorBack
  (params (AxisValue :type Float%20%28double-precision%29))
  (Pawn|Input|AddMovementInput (* (Math|Vector|GetForwardVector (Math|Rotator|MakeRotator (.Roll (Math|Rotator|BreakRotator (Pawn|GetControlRotation :!class /Script/Engine.Pawn))) 0.0 0.0)) (Variables|Default|GetForwardMovingSpeed)) AxisValue false))

(fn MoveRightorLeft
  (params (AxisValue :type Float%20%28single-precision%29))
  (Pawn|Input|AddMovementInput (* (Math|Vector|GetRightVector (Math|Rotator|MakeRotator 0.0 (.Pitch (Math|Rotator|BreakRotator (Pawn|GetControlRotation :!class /Script/Engine.Pawn))) 0.0)) (Variables|Default|GetMoveSpeed)) AxisValue false))

(fn RotateBallMesh
  (params (Delta%20Seconds :type Float%20%28double-precision%29))
  (bind _playermesh (Variables|Default|GetPlayerMesh))
  (bind _output_get (LocalVariables|SetCurrent%20Horizontal%20Velocity (Transformation|GetVelocity)))
  (bind _output_get_2 (LocalVariables|SetCurrent%20Horizontal%20Speed (Math|Vector|VectorLength _output_get)))
  (if (!= _output_get_2 0.0)
    (LocalVariables|SetCurrent%20Rotation%20Amount (* (/ (Math|Vector|VectorLength (LocalVariables|GetCurrent%20Horizontal%20Velocity)) (* (Math|Trig|GetPI) 0.5)) Delta%20Seconds))
    (Transformation|SetRelativeRotation _playermesh (Math|Rotator|CombineRotators (Variables|/Script/Engine.SceneComponent|GetRelativeRotation _playermesh) (Math|Vector|RotatorfromAxisandAngle (Math|Vector|GetRightVector (Math|Rotator|MakeRotfromX (LocalVariables|GetCurrent%20Horizontal%20Velocity))) (LocalVariables|GetCurrent%20Rotation%20Amount))) false false)))